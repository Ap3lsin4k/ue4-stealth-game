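; Functional test that checks a fired projectile spawns with a valid static mesh as its visual representation.
; On test start it waits a zero-length delay, fires the referenced Character, then casts its LastProjectile to BP_Projectile and validates the StaticMesh component.
; It reports success or failure on the mesh check, Invalid when no projectile exists, and Error when the cast fails.
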(event `self.ReceiveStartTest`
  (bind _character (`self.Character`))
  (bind _lastprojectile (`MockFPSCharacter.lastProjectile` _character))
  (`KismetSystemLibrary.Delay` 0.0)
  (`FPSCharacter.Fire` _character)
  (`/Engine/EditorBlueprintResources/StandardMacros.IsValid` _lastprojectile
    (:`Is Valid`
      (bind _asbp_projectile (cast `/Game/Blueprints/BP_Projectile` _lastprojectile)
        (:`then`
          (`/Engine/EditorBlueprintResources/StandardMacros.IsValid` (`/Game/Blueprints/BP_Projectile.StaticMesh` _asbp_projectile)
            (:`Is Valid`
              (`self.FinishTest` "Succeeded" "The projectile has a Visual Representation"))
            (:`Is Not Valid`
              (`self.FinishTest` "Failed" "The projectile has not a valid Visual Representation"))))
        (:`CastFailed`
          (`self.FinishTest` "Error" "Failed to cast to BP Projectile"))))
    (:`Is Not Valid`
      (`self.FinishTest` "Invalid" "The Projectile is Not Valid"))))

(fn `UserConstructionScript`)